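; BP_Car is a car actor that drives itself forward and turns from its Speed and SteeringAngle values.
; Each tick it makes a swept move along its forward vector and yaws in proportion to speed, steering angle and a SpeedToRotation factor.
; It then copies Speed and SteeringAngle to the AB_Car animation instance cached at BeginPlay.
; The event graph contains no input handling.
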(event EventTick
  (params (DeltaSeconds :type Float%20%28single-precision%29))
  (bind _animinstance (Variables|Default|GetAnimInstance))
  ;[1 1 1] Car movement
  (Transformation|AddActorWorldOffset (* DeltaSeconds (* (Transformation|GetActorForwardVector) (Variables|Default|GetSpeed))) true)
  (Class|Actor|AddActorWorldRotation (Math|Rotator|MakeRotator 0.0 0.0 (* (Variables|Default|GetSpeed) (Variables|Default|GetSteeringAngle) (Variables|Default|GetSpeedToRotation) (Utilities|Time|GetWorldDeltaSeconds) 1.5)) true)
  (Utilities|FlowControl|Sequence
    (:then_0
      (Variables|/Game/Blueprints/Car/AB_Car.AB_Car_C|SetSpeed _animinstance (Variables|Default|GetSpeed)))
    (:then_1
      (Variables|/Game/Blueprints/Car/AB_Car.AB_Car_C|SetSteeringAngle _animinstance (Variables|Default|GetSteeringAngle)))))

(event EventBeginPlay
  (bind _asab_car (Utilities|Casting|CastToAB_Car (Components|SkeletalMesh|GetAnimInstance (Variables|Default|GetCar))))
  (Variables|Default|SetAnimInstance _asab_car))

(fn ConstructionScript)