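; Player controller for driving BP_Car: caches the possessed car, adds its input mapping and creates the speed widget.
; Enhanced Input events store throttle, steer and handbrake states and rotate the car's spring arm with clamped pitch.
; Tick eases the car's Speed and SteeringAngle toward input targets using FInterpTo.
; The handbrake zeroes the speed target with faster interpolation and, at high forward speed, enables drifting with extra steering angle.
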(event Input|EnhancedActionEvents|EnhancedInputActionIA_Throttle
  (params (ActionValue :type Float%20%28double-precision%29) (ElapsedSeconds :type Float%20%28double-precision%29) (TriggeredSeconds :type Float%20%28double-precision%29) (InputAction :type Input%20Action%20Object%20Reference :default "/Game/Blueprints/Input/Actions/IA_Throttle.IA_Throttle"))
  ;[1 1 1] Throttle
  (:Triggered
    (Variables|Default|SetbThrottling (Math|Float|Truncate ActionValue)))
  (:Completed
    (Variables|Default|SetbThrottling 0)))

(event Input|EnhancedActionEvents|EnhancedInputActionIA_LookAround
  (params (ActionValue :type Vector%202D%20Structure) (ElapsedSeconds :type Float%20%28double-precision%29) (TriggeredSeconds :type Float%20%28double-precision%29) (InputAction :type Input%20Action%20Object%20Reference :default "/Game/Blueprints/Input/Actions/IA_LookAround.IA_LookAround"))
  ;[1 1 1] Camera rotation
  (:Triggered
    (CallFunction|CameraRotation ActionValue (Variables|/Game/Blueprints/Car/BP_Car.BP_Car_C|GetSpringArm (Variables|Default|GetCar)))))

(event Input|EnhancedActionEvents|EnhancedInputActionIA_Steer
  (params (ActionValue :type Float%20%28double-precision%29) (ElapsedSeconds :type Float%20%28double-precision%29) (TriggeredSeconds :type Float%20%28double-precision%29) (InputAction :type Input%20Action%20Object%20Reference :default "/Game/Blueprints/Input/Actions/IA_Steer.IA_Steer"))
  ;[1 1 1] Steering
  (:Triggered
    (Variables|Default|SetbSteering (Math|Float|Truncate ActionValue)))
  (:Completed
    (Variables|Default|SetbSteering 0)))

(event Input|EnhancedActionEvents|EnhancedInputActionIA_Handbrake
  (params (ActionValue :type Boolean) (ElapsedSeconds :type Float%20%28double-precision%29) (TriggeredSeconds :type Float%20%28double-precision%29) (InputAction :type Input%20Action%20Object%20Reference :default "/Game/Blueprints/Input/Actions/IA_Handbrake.IA_Handbrake"))
  (:Triggered
    (Variables|Default|SetbHandbrake 1))
  (:Completed
    (Variables|Default|SetbHandbrake 0)))

(event EventBeginPlay
  ;[1 1 1] Initialize enhanced input / Other init stuff
  (bind _asbp_player_controller (Utilities|Casting|CastToBP_PlayerController (Game|GetPlayerController 0)))
  (Utilities|IsValid (PlayerController|LocalPlayerSubsystems|GetEnhancedInputLocalPlayerSubsystem _asbp_player_controller)
    (:Is%20Valid
      (Input|AddMappingContext (PlayerController|LocalPlayerSubsystems|GetEnhancedInputLocalPlayerSubsystem _asbp_player_controller) "/Game/Blueprints/Input/IM_Car.IM_Car" 0 "(bIgnoreAllPressedKeysUntilRelease=True,bForceImmediately=False)")
      (bind _returnvalue (UserInterface|CreateWidget "/Game/Blueprints/Widget/BP_Speed.BP_Speed_C" 0 self))
      (UserInterface|Viewport|AddtoViewport _returnvalue 0))))

(event EventTick
  (params (DeltaSeconds :type Float%20%28single-precision%29))
  (bind _car (Variables|Default|GetCar))
  (bind _bthrottling (Variables|Default|GetbThrottling))
  (bind _bsteering (Variables|Default|GetbSteering))
  (bind _returnvalue (Math|Conversions|ToFloat(Integer) _bsteering))
  (bind _returnvalue_2 (Math|Integer|Absolute(Integer) _bsteering))
  (bind _maxsteeringangle (Variables|/Game/Blueprints/Car/BP_Car.BP_Car_C|GetMaxSteeringAngle _car))
  (bind _returnvalue_3 (* _returnvalue_2 _maxsteeringangle))
  ;[1 1 1] Throttle and Steering tick update
  (CallFunction|Throttle (Math|Conversions|ToFloat(Integer) _bthrottling) (* (Math|Integer|Absolute(Integer) _bthrottling) (Variables|/Game/Blueprints/Car/BP_Car.BP_Car_C|GetMaxSpeed (Variables|Default|GetCar)) (- 1 (Variables|Default|GetbHandbrake))))
  (if (Variables|Default|GetbCanDrift)
    (CallFunction|Steering _returnvalue (+ _returnvalue_3 (Variables|Default|GetDriftAdditionalAngles)))
    (else
      (CallFunction|Steering _returnvalue _returnvalue_3))))

(event EventPossess
  (params (PossessedPawn :type Pawn%20Object%20Reference))
  ;[1 1 1] Provide possessed pawn to a variable
  (bind _asbp_car (Utilities|Casting|CastToBP_Car PossessedPawn))
  (Variables|Default|SetCar _asbp_car))

(fn ConstructionScript)

(fn CameraRotation
  (params (Values :type Vector%202D%20Structure) (Actor%20component :type Scene%20Component%20Object%20Reference))
  (Transformation|SetRelativeRotation Actor%20component (Math|Rotator|MakeRotator 0.0 (Math|Float|ClampAngle (+ (.y Values) (.pitch (Variables|/Script/Engine.SceneComponent|GetRelativeRotation Actor%20component))) -75.0 1e+01) (+ (.yaw (Variables|/Script/Engine.SceneComponent|GetRelativeRotation Actor%20component)) (.x Values))) false false))

(fn Throttle
  (params (Value :type Float%20%28double-precision%29) (Target :type Float%20%28double-precision%29))
  (bind _output_get (Variables|/Game/Blueprints/Car/BP_Car.BP_Car_C|SetSpeed (Variables|Default|GetCar) (Math|Interpolation|FInterpTo (Variables|/Game/Blueprints/Car/BP_Car.BP_Car_C|GetSpeed (Variables|Default|GetCar)) (* Value Target) (Utilities|Time|GetWorldDeltaSeconds) (+ (* (LocalVariables|GetHandbrakeFactor) (Variables|Default|GetbHandbrake)) 0.5))))
  (if (>= (* _output_get (Variables|Default|GetbHandbrake)) 1.5e+03)
    (Variables|Default|SetbCanDrift true)
    (else
      (Variables|Default|SetbCanDrift false))))

(fn Steering
  (params (Value :type Float%20%28double-precision%29) (Target :type Float%20%28double-precision%29))
  (Variables|/Game/Blueprints/Car/BP_Car.BP_Car_C|SetSteeringAngle (Variables|Default|GetCar) (Math|Interpolation|FInterpTo (Variables|/Game/Blueprints/Car/BP_Car.BP_Car_C|GetSteeringAngle (Variables|Default|GetCar)) (* Value Target) (Utilities|Time|GetWorldDeltaSeconds) 2.5)))